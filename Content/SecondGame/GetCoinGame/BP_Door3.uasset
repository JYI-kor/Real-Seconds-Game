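; BP_Door3 is a door for the coin game that stays hidden until no BP_Coin2 coins remain in the level.
; On BeginPlay it hides the door and frame meshes and binds to each coin's get-coin dispatcher.
; CoinCheck shows both meshes when RemainCoin, which counts coins not being destroyed, returns zero.
; Only visibility is toggled, with no collision changes.
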(event EventBeginPlay
  (Rendering|SetVisibility (Variables|Default|GetDoor) false false)
  (bind _outactors (Actor|GetAllActorsOfClass "/Game/SecondGame/GetCoinGame/BP_Coin2.BP_Coin2_C"))
  (for _array_element _outactors
    (EventDispatchers|BindEventtoNewEventDispatcherGetCoin _array_element (EventDispatchers|CreateEvent :!event CoinCheck))))

(fn ConstructionScript)

(fn CoinCheck
  (Rendering|SetVisibility (Variables|Default|GetDoor) (== (CallFunction|RemainCoin) 0) false))

(fn RemainCoin
  (bind _outactors (Actor|GetAllActorsOfClass "/Game/SecondGame/GetCoinGame/BP_Coin2.BP_Coin2_C"))
  (for _array_element _outactors
    (if (not (Game|IsActorBeingDestroyed _array_element))
      (LocalVariables|SetCoin (+ (LocalVariables|GetCoin) 1))))
  (return (LocalVariables|GetCoin)))