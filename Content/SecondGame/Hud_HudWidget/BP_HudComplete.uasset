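; HUD controller Blueprint that displays remaining coins and player HP, and sets game-only input with the cursor hidden on BeginPlay.
; It creates HudWidget_Complete, then binds to every BP_Coin2's get-coin dispatcher and BP_PlayerState's HP-update dispatcher, pushing initial values to the widget.
; The remaining-coin count comes from scanning BP_Coin2 actors and skipping any being destroyed.
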(event EventBeginPlay
  (bind _returnvalue (Game|GetPlayerController 0))
  (CallFunction|CreateHudWidget)
  (CallFunction|BindCoin)
  (CallFunction|BindPlayerState)
  (Input|SetInputModeGameOnly _returnvalue false)
  (Variables|/Script/Engine.PlayerController|SetbShowMouseCursor _returnvalue false))

(fn ConstructionScript)

(fn GetCoin
  (Default|ShowCoin (Variables|Default|GetHudWidget)))

(fn HudWidgetShowCoin
  (Default|ShowCoin (Variables|Default|GetHudWidget) (CallFunction|RemainCoin)))

(fn RemainCoin
  (bind _outactors (Actor|GetAllActorsOfClass "/Game/SecondGame/GetCoinGame/BP_Coin2.BP_Coin2_C"))
  (for _array_element _outactors
    (if (not (Game|IsActorBeingDestroyed _array_element))
      (LocalVariables|SetCoin (+ (LocalVariables|GetCoin) 1))))
  (return (LocalVariables|GetCoin)))

(fn CreateHudWidget
  (bind _returnvalue (UserInterface|CreateWidget "/Game/SecondGame/Hud_HudWidget/HudWidget_Complete.HudWidget_Complete_C"))
  (bind _output_get (Variables|Default|SetHudWidget _returnvalue))
  (UserInterface|Viewport|AddtoViewport _output_get 0))

(fn BindCoin
  (bind _outactors (Actor|GetAllActorsOfClass "/Game/SecondGame/GetCoinGame/BP_Coin2.BP_Coin2_C"))
  (for _array_element _outactors
    (EventDispatchers|BindEventtoNewEventDispatcherGetCoin _array_element (EventDispatchers|CreateEvent :!event HudWidgetShowCoin)))
  (CallFunction|HudWidgetShowCoin))

(fn BindPlayerState
  (bind _asbp_player_state (Utilities|Casting|CastToBP_PlayerState (Game|GetPlayerState 0)))
  (EventDispatchers|BindEventtoNewEventDispatcherUpdateHP _asbp_player_state (EventDispatchers|CreateEvent :!event EventUpdateHP))
  (CallFunction|EventUpdateHP (Variables|/Game/SecondGame/GetCoinGame/BP_PlayerState.BP_PlayerState_C|GetCurrent%20HP _asbp_player_state) (Variables|/Game/SecondGame/GetCoinGame/BP_PlayerState.BP_PlayerState_C|GetMax%20HP _asbp_player_state)))

(fn EventUpdateHP
  (params (Current%20HP :type Float%20%28double-precision%29) (Max%20HP :type Float%20%28double-precision%29))
  (Default|UpdateHP (Variables|Default|GetHudWidget) Current%20HP Max%20HP))